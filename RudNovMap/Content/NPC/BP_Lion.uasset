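; Lion NPC that chases the player with AI movement and drives its animation Blueprint's states.
; Each tick feeds the Y component of the normalized direction to the player into the ABP as FacingAngle for run blending.
; Collision events flag the player's approach; the first skips the chase call, later ones start AIMoveTo.
; Reaching the player clears the chasing flags, which comments link to a claw attack, while StopChasing halts movement.
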(event Custom|ChasingPlayer
  (bind _returnvalue (Game|GetPlayerCharacter 0))
  ;[1 1 1] Here you define the main function "ChasingPlayer", which is mainly a translation towards Player`s location. If the player is close, the lion will attack
  (if (Variables|/Game/AfricanAnimalsPack/LionAndLioness/ABP_Lion.ABP_Lion_C|GetIsPlayerApproaching (Variables|Default|GetAs%20ABP%20Lion))
    (Variables|/Game/AfricanAnimalsPack/LionAndLioness/ABP_Lion.ABP_Lion_C|SetIsStillChasing (Variables|Default|GetAs%20ABP%20Lion) true)
    (Variables|Default|SetIsChasing true)
    ;;[0.1397 0.424 0.2515] On Success = IF (AcceptanceRadius <= x) THEN the lion performs "Run" -> "ClawsAttack"
    (AI|AIMoveTo self (Transformation|GetActorLocation _returnvalue) _returnvalue 1e+01 false
      (:OnSuccess
        (Variables|Default|SetIsChasing false)
        (Variables|/Game/AfricanAnimalsPack/LionAndLioness/ABP_Lion.ABP_Lion_C|SetIsStillChasing (Variables|Default|GetAs%20ABP%20Lion) false)))))

(event Custom|WhileOnCollision
  ;[1 1 1] The use of "FirstTime?" discirminates which animation to perform: a) Rest -> GetUp -> Run OR b) EnGarde -> Run
  (Variables|/Game/AfricanAnimalsPack/LionAndLioness/ABP_Lion.ABP_Lion_C|SetIsPlayerApproaching (Variables|Default|GetAs%20ABP%20Lion) true)
  (if (Variables|Default|GetFirstTime?)
    (Variables|Default|SetFirstTime? false)
    (else
      (CallFunction|ChasingPlayer))))

(event Custom|StopChasing
  ;[1 1 1] When the player is out of the trigger box, the running animation and the movement are stopped
  (Variables|/Game/AfricanAnimalsPack/LionAndLioness/ABP_Lion.ABP_Lion_C|SetIsPlayerApproaching (Variables|Default|GetAs%20ABP%20Lion) false)
  (Class|NavMovementComponent|StopActiveMovement (Variables|Character|GetCharacterMovement)))

(event EventBeginPlay
  ;[1 0.4764 0.07479] This directly access the animation graph
  (Variables|Default|SetFirstTime? true)
  (bind _asabp_lion (Utilities|Casting|CastToABP_Lion (Components|SkeletalMesh|GetAnimInstance (Variables|Character|GetMesh))))
  (Variables|Default|SetAs%20ABP%20Lion _asabp_lion))

(event EventTick
  (params (DeltaSeconds :type Float%20%28single-precision%29))
  ;[1 1 1] Every frame, I calculate the direction in which the lion would run: this influences in the blend space in the ABP the animation to perform (run straight, left or right)
  (Variables|/Game/AfricanAnimalsPack/LionAndLioness/ABP_Lion.ABP_Lion_C|SetFacingAngle (Variables|Default|GetAs%20ABP%20Lion) (.Y (Math|Vector|BreakVector (Math|Vector|Normalize (- (Transformation|GetActorLocation (Game|GetPlayerCharacter 0)) (Transformation|GetActorLocation)))))))

(fn ConstructionScript)